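; BP_Useable is an interactable world item, currently a flashlight ("Linterna"), that the player can pick up.
; DT_ItemsData supplies the mesh from a hard-coded "Linterna" row in construction, and the prompt texts from the TipoDeObjeto row at BeginPlay.
; Box overlaps and interaction-interface states animate the WBP_Interact prompt, which turns toward the camera each tick.
; A successful interaction calls IniciarRecogida on BP_Player, passing the item's location and itself as the actor to destroy.
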(event OnComponentBeginOverlap(Box)
  (params (OverlappedComponent :type Primitive%20Component%20Object%20Reference) (OtherActor :type Actor%20Object%20Reference) (OtherComp :type Primitive%20Component%20Object%20Reference) (OtherBodyIndex :type Integer) (bFromSweep :type Boolean) (SweepResult :type Hit%20Result%20Structure%20%28by%20ref%29))
  (Utilities|Casting|CastToBP_Player OtherActor)
  (Default|AnimarMostrar (Variables|Default|GetAs%20WBP%20Interact)))

(event OnComponentEndOverlap(Box)
  (params (OverlappedComponent :type Primitive%20Component%20Object%20Reference) (OtherActor :type Actor%20Object%20Reference) (OtherComp :type Primitive%20Component%20Object%20Reference) (OtherBodyIndex :type Integer))
  (Utilities|Casting|CastToBP_Player OtherActor)
  (Default|AnimarNoMostrar (Variables|Default|GetAs%20WBP%20Interact)))

(event EventBeginPlay
  (Utilities|FlowControl|Sequence
    (:then_0
      (bind _aswbp_interact (Utilities|Casting|CastToWBP_Interact (UserInterface|GetUserWidgetObject (Variables|Default|GetWidget))))
      (bind _output_get (Variables|Default|SetAs%20WBP%20Interact _aswbp_interact))
      (Class|BPIInteractData|ObtenerTextosUI(Message) _output_get)
      (Default|AnimarNoMostrar (Variables|Default|GetAs%20WBP%20Interact)))
    (:then_1
      (bind _returnvalue (Utilities|GetDataTableRow "/Game/InteractSystem/DT_ItemsData.DT_ItemsData" (Utilities|String|StringToName (Utilities|String|EnumtoString (Variables|Components|GetTipoDeObjeto))))
        (:then
          (Default|ActualizarTextosUI (Variables|Default|GetAs%20WBP%20Interact) (.TextoUI (Utilities|Struct|BreakS_ItemInfo _returnvalue)) (.TeclaUI (Utilities|Struct|BreakS_ItemInfo _returnvalue))))))))

(event Collision|EventActorBeginOverlap
  (params (OtherActor :type Actor%20Object%20Reference)))

(event EventTick
  (params (DeltaSeconds :type Float%20%28single-precision%29))
  (Transformation|SetWorldRotation (Variables|Default|GetWidget) (Math|Rotator|FindLookatRotation (Transformation|GetActorLocation) (Camera|GetCameraLocation (Game|GetPlayerCameraManager 0))) false false))

(event EventOnInteractionStateChangedBPI
  (params (State :type E_InteractionState%20Enum :default "Pre") (Interactor :type Pawn%20Object%20Reference))
  (bind _as_wbp_interact (Variables|Default|GetAs%20WBP%20Interact))
  (switch Utilities|FlowControl|Switch|SwitchonE_InteractionState State
    (:Pre
      (Default|AnimarMostrar _as_wbp_interact))
    (:Fail
      (Default|AnimarNoMostrar _as_wbp_interact))
    (:Succeed
      (bind _asbp_player (Utilities|Casting|CastToBP_Player Interactor))
      (switch Utilities|FlowControl|Switch|SwitchonE_TipoObjeto "NewEnumerator0"
        (:NewEnumerator0
          (Default|IniciarRecogida _asbp_player (Transformation|GetActorLocation) self))))))

(fn ConstructionScript
  (bind _returnvalue (Utilities|GetDataTableRow "/Game/InteractSystem/DT_ItemsData.DT_ItemsData" "Linterna")
    (:then
      (Components|StaticMesh|SetStaticMesh (Variables|Default|GetStaticMesh) (.mallavisual _returnvalue)))
    (:RowNotFound
      (Development|PrintString "not ofcund"))))

(fn CanInteractBPI
  (params (Interactor :type Pawn%20Object%20Reference))
  (return true))

(fn OpenCustomDepthBPI
  (params (Open :type Boolean))
  (return false))